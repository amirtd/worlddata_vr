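; BP_Data_actor is an actor that reads one city's record from the Worldcities_Datatable and prints it on screen, apparently as a data table lookup test.
; On BeginPlay it fetches the hardcoded "Tokyo" row.
; If the row is found, it stores the city, ASCII name, latitude, longitude and country in variables, printing each in turn.
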(event EventBeginPlay
  (bind _returnvalue (Utilities|GetDataTableRow "/Game/worldcities_Datatable.worldcities_Datatable" "Tokyo")
    (:then
      (Utilities|FlowControl|Sequence
        (:then_0
          (bind _output_get (Variables|Default|SetCity (.city (Utilities|Struct|BreakCity_Struct _returnvalue))))
          (Development|PrintString (Utilities|String|ToString(Name) _output_get)))
        (:then_1
          (bind _output_get_2 (Variables|Default|SetCity%20String (.city_ascii (Utilities|Struct|BreakCity_Struct _returnvalue))))
          (Development|PrintString (Utilities|String|ToString(Name) _output_get_2)))
        (:then_2
          (bind _output_get_3 (Variables|Default|SetLattitute (.lat (Utilities|Struct|BreakCity_Struct _returnvalue))))
          (Development|PrintString (Utilities|String|ToString(Float) _output_get_3)))
        (:then_3
          (bind _output_get_4 (Variables|Default|SetLongtitute (.lng (Utilities|Struct|BreakCity_Struct _returnvalue))))
          (Development|PrintString (Utilities|String|ToString(Float) _output_get_4)))
        (:then_4
          (bind _output_get_5 (Variables|Default|SetCoutnry (.Country (Utilities|Struct|BreakCity_Struct _returnvalue))))
          (Development|PrintString (Utilities|String|ToString(Name) _output_get_5)))))))

(fn ConstructionScript)